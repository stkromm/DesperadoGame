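; Dropped-item actor that displays a mesh and merges into nearby drops on BeginPlay.
; A sphere trace within StackDistance finds another Drop, adds item amounts to its Storage, sets a Despawn timer on that Storage, resizes it and destroys itself.
; If the trace hits nothing, it spawns a ListInventory as its own Storage.
; SetSize scales the mesh by capacity over used capacity, so fuller storage gives a smaller mesh.
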(event `self.ReceiveBeginPlay`
  (bind _returnvalue (`self.K2_GetActorLocation`))
  (`StaticMeshComponent.SetStaticMesh` (`self.StaticMesh`) (`self.Mesh`))
  (bind (_outhits _returnvalue_2) (`KismetSystemLibrary.SphereTraceMultiForObjects` :`Start` _returnvalue :`End` (+ _returnvalue (0.0 0.0 1.0)) :`Radius` (`self.StackDistance`) :`ObjectTypes` (`|MakeArray` "ObjectTypeQuery2" "ObjectTypeQuery1" :!type "EObjectTypeQuery Enum") :`DrawDebugType` "ForDuration"))
  (if _returnvalue_2
    (for _array_element _outhits
      (bind _asdrop (cast `/Game/Blueprints/Drop` (`.HitActor` (`GameplayStatics.BreakHitResult` _array_element))))
      (for _array_element_2 _
        (bind _storage (`/Game/Blueprints/Drop.Storage` _asdrop))
        (bind (_amount _identifier) (break `ItemAmount` _array_element_2))
        (`AbstractInventory.AddAmount` _storage _amount _identifier))
      (`KismetSystemLibrary.K2_SetTimer` _storage "Despawn" (`self.DespawnLength`))
      (`self.SetSize` _asdrop)
      (`self.K2_DestroyActor`)
      (break))
    (else
      (bind _returnvalue_3 (`|SpawnActorFromClass` "/Script/MyProject.ListInventory" (`self.GetTransform`) "Undefined" "OverrideRootScale" null 1000))
      (set `self.Storage` _returnvalue_3))))

(event `self.ReceiveActorBeginOverlap`
  (params (OtherActor :type "Actor Object Reference")))

(fn `Despawn`
  (`self.K2_DestroyActor`))

(fn `SetSize`
  (bind _storage (`self.Storage`))
  (`SceneComponent.SetWorldScale3D` (`self.StaticMesh`) (* (0.5 0.5 0.5) (+ (/ (`KismetMathLibrary.Conv_IntToDouble` (`ListInventory.Capacity` _storage)) (`KismetMathLibrary.Conv_IntToDouble` (`ListInventory.GetUsedCapacity` _storage))) 1.0))))

(fn `UserConstructionScript`)