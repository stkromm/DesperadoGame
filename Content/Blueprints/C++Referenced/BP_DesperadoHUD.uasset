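; Desperado HUD Blueprint that owns the player's inventory screen and toggles it on and off.
; BeginPlay creates the W_Inventory widget for the owning player controller and stores it.
; ToggleInventory adds the widget to the viewport on first use, then switches between Visible and Collapsed rather than removing it.
; Showing it sets UI-only input focused on the inventory with the mouse locked to the viewport, while hiding it restores game-only input.
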(event `self.ReceiveBeginPlay`
  (bind _returnvalue (`|CreateWidget` "/Game/Blueprints/Widgets/W_Inventory.W_Inventory_C" (`self.GetOwningPlayerController`)))
  (set `self.Inventory` _returnvalue))

(event `self.ReceiveActorBeginOverlap`
  (params (OtherActor :type "Actor Object Reference")))

(event `self.ReceiveTick`
  (params (DeltaSeconds :type "Float (single-precision)")))

(event `self.ToggleInventory`
  (bind _inventory (`self.Inventory`))
  (if (`Widget.IsInViewport` _inventory)
    (if (`Widget.IsVisible` _inventory)
      (`Widget.SetVisibility` _inventory "Collapsed")
      (`WidgetBlueprintLibrary.SetInputMode_GameOnly` null)
      (else
        (`Widget.SetVisibility` _inventory "Visible" :!label _label)
        (`WidgetBlueprintLibrary.SetInputMode_UIOnlyEx` null _inventory true)))
    (else
      (`UserWidget.AddToViewport` _inventory 0)
      (goto _label))))

(fn `UserConstructionScript`)